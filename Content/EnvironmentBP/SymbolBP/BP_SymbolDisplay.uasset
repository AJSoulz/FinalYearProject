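; BP_SymbolDisplay is a segmented symbol display that shows the combined pattern of its DoorKeys.
; BeginPlay XORs each key's SegmentDisplay array into its own, element by element, then writes each result to a material scalar parameter named by its index.
; The construction script creates that dynamic material instance on the Cube.
; BeginPlay also prints a hard-coded XOR of three large integers.
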(event `self.ReceiveBeginPlay`
  (`KismetSystemLibrary.PrintString` (`KismetTextLibrary.Conv_TextToString` (`KismetTextLibrary.Conv_Int64ToText` (`KismetMathLibrary.Xor_Int64Int64` (`KismetMathLibrary.Xor_Int64Int64` 282134969974818 281842339545241) 431594384942592))) true true (struct :`G` 0.66 :`B` 1.0 :`A` 1.0) 20.0)
  ;[0 0.00025 0.2188 1 12] Perform XOR operation on each DoorKey.
  (for _array_element (`self.DoorKeys`)
    (for (_array_element_2 _array_index) (`/Game/EnvironmentBP/SymbolBP/BP_DoorKey.SegmentDisplay` _array_element)
      (`KismetArrayLibrary.Array_Set` (`self.SegmentDisplay`) _array_index (xor _array_element_2 (`|GetArrayItem` (`self.SegmentDisplay`) _array_index)) true)))
  ;[0 0.00025 0.2188 1 12] Update material parameters.
  (for (_array_element_3 _array_index_2) (`self.SegmentDisplay`)
    (`MaterialInstanceDynamic.SetScalarParameterValue` (`self.DMI`) (`KismetStringLibrary.Conv_StringToName` (`KismetStringLibrary.Conv_IntToString` _array_index_2)) (`KismetMathLibrary.Conv_BoolToDouble` _array_element_3))))

(fn `UserConstructionScript`
  ;[0 0.00025 0.2188 1 12] Create dynamic material instance.
  (bind _returnvalue (`KismetMaterialLibrary.CreateDynamicMaterialInstance` (`PrimitiveComponent.GetMaterial` (`self.Cube`) 0)))
  (bind _output_get (set `self.DMI` _returnvalue))
  (`PrimitiveComponent.SetMaterial` (`self.Cube`) 0 _output_get))