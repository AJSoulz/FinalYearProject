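; BP_DiscSpawnPad is a pad that spawns puzzle discs for the disc puzzle.
; On BeginPlay it looks up its row in DT_PuzzleDisc and replaces its actor tags with that row's ID.
; RespawnDisc spawns a flattened BP_PuzzleDisc just above the pad regardless of collision, passing on the same row name.
; The file never calls RespawnDisc itself, nor removes any existing disc.
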(event `self.ReceiveBeginPlay`
  (bind _returnvalue (`|GetDataTableRow` "/Game/Objects/Dynamic/PuzzleDisc/Base/Blueprint/DT_PuzzleDisc.DT_PuzzleDisc" (`self.Data Table Row`))
    (:`then`
      (set `self.Tags` (`|MakeArray` (`.ID_50_DEE222C7444A4711C8270282DCEC79DA` (break `/Game/Objects/Dynamic/PuzzleDisc/Base/Blueprint/Struct_PuzzleDisc` _returnvalue)))))))

(event `/Game/Objects/Dynamic/PuzzleDiscSpawn/Blueprint/BPI_DiscRespawn.Respawn Disc`
  (`|SpawnActorFromClass` "/Game/Objects/Dynamic/PuzzleDisc/Base/Blueprint/BP_PuzzleDisc.BP_PuzzleDisc_C" (`KismetMathLibrary.MakeTransform` (`KismetMathLibrary.MakeVector` (.x (`self.K2_GetActorLocation` self)) (.y (`self.K2_GetActorLocation` self)) (+ (.z (`self.K2_GetActorLocation` self)) 7.0)) (struct) (0.2 0.2 1.0)) "AlwaysSpawn" "OverrideRootScale" null (`self.Data Table Row`) null))

(fn `UserConstructionScript`)