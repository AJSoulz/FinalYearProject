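; Puzzle doorway that dematerialises when the discs placed in its slots combine to match the target value from its row in DT_DoorData.
; Each slot gets a reference to the door at BeginPlay, and each symbol update refreshes that slot's line and dot textures on the output material.
; The disc values are XORed against the target: a match plays a dissolve timeline that drops collision partway through, otherwise it reverses.
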(event `self.ReceiveBeginPlay`
  (`|ExecutionSequence`
    (:`then_0`
      (for (_ _array_index) (`self.Disc Slots`)
        (`/Game/Objects/Dynamic/PuzzleDoor/PuzzleDoorBP/BP_DoorDiscSlot.Set Doorway Reference` (`|GetArrayItem` (`self.Disc Slots`) _array_index) self _array_index)))
    (:`then_1`
      (bind _returnvalue (`|GetDataTableRow` "/Game/Objects/Dynamic/PuzzleDoor/PuzzleDoorBP/DT_DoorData.DT_DoorData" (`self.Data Table Row`))
        (:`then`
          (bind _output_get (set `self.Door Puzzle Data` _returnvalue))
          (`MaterialInstanceDynamic.SetTextureParameterValue` (`self.DMI Puzzle Hint`) "Symbol Texture" (`.SymbolTexture_12_FC9F19EC48B896CA0DD401B193F70875` (break `/Game/Objects/Dynamic/PuzzleDoor/PuzzleDoorBP/S_DoorPuzzle` _output_get))))
        (:`RowNotFound`
          (`KismetSystemLibrary.PrintString` (`KismetStringLibrary.Concat_StrStr` (`KismetSystemLibrary.GetObjectName` self) "  -  Data table row not found") true false (struct :`R` 1.0 :`B` 0.015913 :`A` 1.0) 10.0))))))

(event `/Game/Objects/Dynamic/PuzzleDoor/PuzzleDoorBP/BPI_DoorUpdate.Update Symbol Output`
  (params (`Is Empty?` :type Boolean) (`Slot Number` :type Integer))
  (`|ExecutionSequence`
    (:`then_0`
      (`self.Update Material Instance` `Is Empty?` `Slot Number`))
    (:`then_1`
      (`PrimitiveComponent.SetCollisionEnabled` (`self.Door (Collision)`) "QueryAndPhysics")
      (bind _is_solved_ (`self.Puzzle Solved?`))
      (if _is_solved_
        (bind (_direction _main_door_dissolve_amount _adornment_dissolve_amount) (`Timeline|Dematerialise` :!label _label)
          (:`Update`
            (`MaterialInstanceDynamic.SetScalarParameterValue` (`self.DMI Main Door`) "Dissolve Amount" _main_door_dissolve_amount)
            (`MaterialInstanceDynamic.SetScalarParameterValue` (`self.DMI Symbol Output`) "Dissolve Amount" _adornment_dissolve_amount)
            (`MaterialInstanceDynamic.SetScalarParameterValue` (`self.DMI Puzzle Hint`) "Dissolve Amount" _adornment_dissolve_amount)
            (if (and (>= _main_door_dissolve_amount 30.0) (`|EnumEquality` _direction "Forward"))
              (`PrimitiveComponent.SetCollisionEnabled` (`self.Door (Collision)`) "NoCollision"))))
        (else
          (goto _label :!via `Reverse`))))))

(fn `Puzzle Solved?`
  (returns (`Is Solved?` :type Boolean))
  (locals (`Running Puzzle Value` :type Integer64))
  (for (_ _array_index) (`self.Disc Slots`)
    (set `local.Running Puzzle Value` (`KismetMathLibrary.Xor_Int64Int64` (`local.Running Puzzle Value`) (`.PuzzleValue_40_1014FD784AA2D9D6B2693F843D53E481` (break `/Game/Objects/Dynamic/PuzzleDisc/Base/Blueprint/Struct_PuzzleDisc` (`/Game/Objects/Dynamic/PuzzleDoor/PuzzleDoorBP/BP_DoorDiscSlot.Disc Data` (`|GetArrayItem` (`self.Disc Slots`) _array_index)))))))
  (return (== (`local.Running Puzzle Value`) (`.PuzzleValue_10_37564E3648834452D3495B81CC01D3F8` (break `/Game/Objects/Dynamic/PuzzleDoor/PuzzleDoorBP/S_DoorPuzzle` (`self.Door Puzzle Data`))))))

(fn `Update Material Instance`
  (params (`Empty?` :type Boolean) (`Slot Number` :type Integer))
  (bind _returnvalue (`KismetStringLibrary.Conv_IntToString` `Slot Number`))
  (bind ((`SymbolOnlyLines_44_F9701ED048A1D3A1846489A7424A2D9D` _symbolonlylines) (`SymbolOnlyDots_46_AF5830A74354B087649995B625CAAEEE` _symbolonlydots)) (break `/Game/Objects/Dynamic/PuzzleDisc/Base/Blueprint/Struct_PuzzleDisc` (`/Game/Objects/Dynamic/PuzzleDoor/PuzzleDoorBP/BP_DoorDiscSlot.Disc Data` (`|GetArrayItem` (`self.Disc Slots`) `Slot Number`))))
  (if `Empty?`
    (set `self.Texture (Only Lines)` "/Game/Objects/Dynamic/PuzzleDisc/Symbol/Texture/T_Symbol_0000000000000.T_Symbol_0000000000000")
    (set `self.Texture (Only Dots)` "/Game/Objects/Dynamic/PuzzleDisc/Symbol/Texture/T_Symbol_0000000000000.T_Symbol_0000000000000")
    (else
      (set `self.Texture (Only Lines)` _symbolonlylines)
      (set `self.Texture (Only Dots)` _symbolonlydots)))
  (`MaterialInstanceDynamic.SetTextureParameterValue` (`self.DMI Symbol Output`) (`KismetStringLibrary.Conv_StringToName` (`KismetStringLibrary.Concat_StrStr` "Lines" _returnvalue)) (`self.Texture (Only Lines)`))
  (`MaterialInstanceDynamic.SetTextureParameterValue` (`self.DMI Symbol Output`) (`KismetStringLibrary.Conv_StringToName` (`KismetStringLibrary.Concat_StrStr` "Dots" _returnvalue)) (`self.Texture (Only Dots)`)))

(fn `UserConstructionScript`
  (bind _returnvalue (`PrimitiveComponent.CreateDynamicMaterialInstance` (`self.Symbol Feedback (Mesh)`) 0 "/Game/Objects/Dynamic/PuzzleDoor/DoorMaterials/M_DoorSymbolOutput.M_DoorSymbolOutput" "None"))
  (set `self.DMI Symbol Output` _returnvalue)
  (bind _returnvalue_2 (`PrimitiveComponent.CreateDynamicMaterialInstance` (`self.Cube (Mesh)`) 0 "/Game/Objects/Dynamic/PuzzleDoor/DoorMaterials/MI_Dematerialise.MI_Dematerialise" "None"))
  (set `self.DMI Main Door` _returnvalue_2)
  (bind _returnvalue_3 (`PrimitiveComponent.CreateDynamicMaterialInstance` (`self.Puzzle Hint (Mesh)`) 0 "/Game/Objects/Dynamic/PuzzleDoor/DoorMaterials/M_DoorHint.M_DoorHint" "None"))
  (set `self.DMI Puzzle Hint` _returnvalue_3))