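; Puzzle disc pickup that the first-person player collects into their inventory.
; BeginPlay loads its data table row, sets both symbol materials, and plays a rise, scale and spin timeline before enabling overlap and starting a pulsing, bobbing animation.
; On player overlap it sends its item data to the player and to all skeletons tagged with the disc's ID, which get back up, then destroys itself.
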(event `self.ReceiveBeginPlay`
  (bind _start_location (`self.Start Location`))
  (set `PrimitiveComponent.bGenerateOverlapEvents` false (`self.SphereCollision`))
  (bind _returnvalue (`|GetDataTableRow` "/Game/Objects/Dynamic/PuzzleDisc/Base/Blueprint/DT_PuzzleDisc.DT_PuzzleDisc" (`self.Data Table Row`))
    (:`then`
      (bind _output_get (set `self.ItemData` _returnvalue))
      (bind ((`MaterialInstance_41_B9B57ED740E93DD13ED561B720CFAD3D` _materialinstance)) (break `/Game/Objects/Dynamic/PuzzleDisc/Base/Blueprint/Struct_PuzzleDisc` _output_get))
      (`PrimitiveComponent.SetMaterial` (`self.Symbol Obverse`) 0 _materialinstance)
      (`PrimitiveComponent.SetMaterial` (`self.Symbol Reverse`) 0 _materialinstance)
      (set `self.Start Location` (`self.K2_GetActorLocation`))
      (bind (_direction _height _scale _rotation) (`Timeline|Respawn Animation`)
        (:`Update`
          (`self.K2_SetActorLocation` (`KismetMathLibrary.VLerp` _start_location (+ _start_location (0.0 0.0 125.0)) _height))
          (`self.SetActorScale3D` (`KismetMathLibrary.MakeVector` _scale _scale (.z (`self.GetActorScale3D`))))
          (`self.K2_SetActorRotation` (`KismetMathLibrary.RLerp` (struct) (struct :`Yaw` 585.0 :`Roll` 45.0) _rotation)))
        (:`Finished`
          (set `PrimitiveComponent.bGenerateOverlapEvents` true (`self.SphereCollision`))
          (bind (_direction_2 _offset _rotate _bobbing) (`Timeline|Pulse`)
            (:`Update`
              (`SceneComponent.SetRelativeScale3D` (`self.Mesh Depth`) (`KismetMathLibrary.MakeVector` (.x (`SceneComponent.K2_GetComponentScale` (`self.Mesh Depth`))) (.y (`SceneComponent.K2_GetComponentScale` (`self.Mesh Depth`))) _offset))
              (`SceneComponent.K2_SetRelativeRotation` (`self.Mesh Depth`) (`KismetMathLibrary.RLerp` (struct) (struct :`Yaw` 90.0) _rotate) false false)
              (`SceneComponent.K2_SetRelativeRotation` (`self.Mesh Edge`) (`KismetMathLibrary.RLerp` (struct) (struct :`Yaw` -90.0) _rotate) false false)
              (`self.K2_SetActorLocation` (`KismetMathLibrary.MakeVector` (.x (`self.K2_GetActorLocation`)) (.y (`self.K2_GetActorLocation`)) (+ (.z (`self.K2_GetActorLocation`)) _bobbing))))))))))

(event `self.SphereCollision.OnComponentBeginOverlap`
  (params (OverlappedComponent :type "PrimitiveComponent Object Reference") (OtherActor :type "Actor Object Reference") (OtherComp :type "PrimitiveComponent Object Reference") (OtherBodyIndex :type Integer) (bFromSweep :type Boolean) (SweepResult :type "HitResult Structure (by ref)"))
  (bind _itemdata (`self.ItemData`))
  (bind _asfirst_person_character (cast `/Game/Character/Player/Blueprint/FirstPersonCharacter` OtherActor)) ; Ensure that it is picked up by the player.
  (message `/Game/Objects/Dynamic/PuzzleDisc/Base/Blueprint/BPI_ItemPickup.OnItemPickup` _asfirst_person_character _itemdata) ; Notify FirstPersonCharacter.\nWill add this PuzzleDisc to the player inventory.
  (bind _outactors (`GameplayStatics.GetAllActorsOfClassWithTag` "/Game/Character/Enemy/EnemySkeleton/BP_Skeleton.BP_Skeleton_C" (`.ID_50_DEE222C7444A4711C8270282DCEC79DA` (break `/Game/Objects/Dynamic/PuzzleDisc/Base/Blueprint/Struct_PuzzleDisc` _itemdata))))
  (message `/Game/Objects/Dynamic/PuzzleDisc/Base/Blueprint/BPI_ItemPickup.OnItemPickup` _outactors (`self.ItemData`)) ; Notify all Skeletons downed by this disc. \nThey will all get back up.
  (`self.K2_DestroyActor`))

(event `self.ReceiveTick`
  (params (DeltaSeconds :type "Float (single-precision)")))

(fn `UserConstructionScript`)