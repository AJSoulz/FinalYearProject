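; BP_InventorySystem is an inventory component that currently detects what the player looks at for interaction.
; Each tick it sphere-traces from the camera along its forward vector up to InteractionRange, ignoring its owner.
; When the hit actor changes, it caches it as LookedAtActor and prints its LookAtMessage result; a miss clears it.
; AddToInventory and RemoveFromInventory are empty stubs.
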(event `self.ReceiveTick`
  (params (DeltaSeconds :type "Float (single-precision)"))
  (`self.TraceForInteraction`))

(fn `AddToInventory`)

(fn `RemoveFromInventory`)

(fn `TraceForInteraction`
  (bind _returnvalue (`GameplayStatics.GetPlayerCameraManager` 0))
  (bind _returnvalue_2 (`PlayerCameraManager.GetCameraLocation` _returnvalue))
  (bind (_outhit _returnvalue_3) (`KismetSystemLibrary.SphereTraceSingle` _returnvalue_2 (+ _returnvalue_2 (* (`Actor.GetActorForwardVector` _returnvalue) (`self.InteractionRange`))) 15.0 "TraceTypeQuery3" false (`|MakeArray` (`self.GetOwner`))))
  (if _returnvalue_3
    (bind (_bblockinghit _binitialoverlap _time _distance _location _impactpoint _normal _impactnormal _physmat _hitactor) (`GameplayStatics.BreakHitResult` _outhit))
    (if (!= (`self.LookedAtActor`) _hitactor)
      (bind _output_get (set `self.LookedAtActor` _hitactor))
      (bind _message (message `/Game/Inventory/I_Interactive.LookAt` _output_get))
      (`KismetSystemLibrary.PrintString` (`KismetTextLibrary.Conv_TextToString` _message)))
    (else
      (set `self.LookedAtActor` null))))