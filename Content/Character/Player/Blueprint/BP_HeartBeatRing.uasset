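; BP_HeartBeatRing is an expanding-ring actor, driven by a heartbeat interval, that alerts skeleton enemies it touches.
; The Scale timeline animates a flattened cylinder's size and dynamic-material opacity, then destroys the actor.
; LastIBI sets both playback rate and clamped size, so shorter intervals give larger, slower rings.
; Overlapping a BP_EnemySkeleton switches its AIC_EnemySkeleton controller to attacking, passing the ring itself.
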(event `self.ReceiveBeginPlay`
  (`TimelineComponent.SetPlayRate` (`self.Scale`) (* (`self.LastIBI`) 4.0))
  (bind (_direction _scale _opacity) (`Timeline|Scale`)
    (:`Update`
      (bind _returnvalue (* (`KismetMathLibrary.FClamp` (- 10.0 (* (`self.LastIBI`) 8.0)) 1.0 10.0) _scale))
      (`SceneComponent.SetWorldScale3D` (`self.Cylinder`) (`KismetMathLibrary.MakeVector` _returnvalue _returnvalue 0.01))
      (`MaterialInstanceDynamic.SetScalarParameterValue` (`self.Dynamic Material Instance`) "Opacity" _opacity))
    (:`Finished`
      (`self.K2_DestroyActor`))))

(event `self.Cylinder.OnComponentBeginOverlap`
  (params (OverlappedComponent :type "PrimitiveComponent Object Reference") (OtherActor :type "Actor Object Reference") (OtherComp :type "PrimitiveComponent Object Reference") (OtherBodyIndex :type Integer) (bFromSweep :type Boolean) (SweepResult :type "HitResult Structure (by ref)"))
  (bind _asbp_enemy_skeleton (cast `/Game/Character/Enemy/EnemySkeleton/Blueprint/BP_EnemySkeleton` OtherActor))
  (bind _asaic_enemy_skeleton (cast `/Game/Character/Enemy/EnemySkeleton/AI/AIC_EnemySkeleton` (`AIBlueprintHelperLibrary.GetAIController` _asbp_enemy_skeleton)))
  (`/Game/Character/Enemy/EnemySkeleton/AI/AIC_EnemySkeleton.Set State As Attacking` _asaic_enemy_skeleton self))

(fn `UserConstructionScript`
  (bind _returnvalue (`PrimitiveComponent.CreateDynamicMaterialInstance` (`self.Cylinder`) 0 "/Game/Character/Player/Material/M_Ring.M_Ring" "None"))
  (set `self.Dynamic Material Instance` _returnvalue))