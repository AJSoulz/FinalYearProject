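; BP_EnemySkeleton is a skeleton enemy character that patrols and deals sword damage to the player.
; Sword anim notifies reset a per-swing flag, then check the sword collision for player overlap, applying normal and permanent lunge damage once per attack.
; Helper functions expose the patrol route and map idle, walking and running states to max walk speed.
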(event `self.ReceiveBeginPlay`
  (bind _asfirst_person_character (cast `/Game/Character/Player/Blueprint/FirstPersonCharacter` (`GameplayStatics.GetPlayerCharacter` 0)))
  (set `self.Player Reference` _asfirst_person_character))

(event `/Game/Character/Enemy/EnemySkeleton/Blueprint/BPI_AnimNotify.(Anim Notify) New Sword Attack`
  (set `self.Has Damage Been Applied?` false))

(event `/Game/Character/Enemy/EnemySkeleton/Blueprint/BPI_AnimNotify.(Anim Notify) Sword Collision Check`
  (if (and (not (`self.Has Damage Been Applied?`)) (`PrimitiveComponent.IsOverlappingActor` (`self.Sword Damage Collision`) (`GameplayStatics.GetPlayerCharacter` 0)))
    (set `self.Has Damage Been Applied?` true)
    (`/Game/Character/Player/Blueprint/FirstPersonCharacter.Apply Damage` (`self.Player Reference`) (`self.LUNGE ATTACK NORMAL DAMAGE`) (`self.LUNGE ATTACK PERMANENT DAMAGE`))))

(fn `Get Patrol Route`
  (returns (`Patrol Route` :type "/Game/Character/Enemy/EnemySkeleton/AI/BP_PatrolRoute Object Reference"))
  (return (`self.Patrol Route`)))

(fn `Set Movement Speed`
  (params (`Movement Speed` :type "/Game/Character/Enemy/EnemySkeleton/AI/E_MovementSpeed Enum" :default "NewEnumerator2"))
  (returns (`Speed Value` :type "Float (double-precision)"))
  (bind _output_get (set `CharacterMovementComponent.MaxWalkSpeed` (select `/Game/Character/Enemy/EnemySkeleton/AI/E_MovementSpeed` `Movement Speed` :`NewEnumerator0` 45.0 :`NewEnumerator1` 375.0 :!type "Float (single-precision)") (`self.CharacterMovement`)))
  (return _output_get))

(fn `UserConstructionScript`)