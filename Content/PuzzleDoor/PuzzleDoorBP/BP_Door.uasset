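; BP_Door is a puzzle door with three child disc slots (left, centre, right) whose combined values must match a passcode.
; BeginPlay caches each slot and assigns its position name.
; UpdateSymbolOutput writes line and dot textures to position-named parameters on a dynamic symbol material, then checks the answer.
; The check XORs the three disc puzzle values against DoorPasscode; success only shows a debug message, with no opening logic.
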(event `self.ReceiveBeginPlay`
  (bind _asbp_door_disc_slot (cast `/Game/PuzzleDoor/PuzzleDoorBP/BP_DoorDiscSlot` (`ChildActorComponent.ChildActor` (`self.(Child Actor) Disc Slot Left`))))
  (bind _output_get (set `self.Disc (Left)` _asbp_door_disc_slot))
  (set `/Game/PuzzleDoor/PuzzleDoorBP/BP_DoorDiscSlot.Left / Centre / Right` "Left" _output_get)
  (bind _asbp_door_disc_slot_2 (cast `/Game/PuzzleDoor/PuzzleDoorBP/BP_DoorDiscSlot` (`ChildActorComponent.ChildActor` (`self.(Child Actor) Disc Slot Centre`))))
  (bind _output_get_2 (set `self.Disc (Centre)` _asbp_door_disc_slot_2))
  (set `/Game/PuzzleDoor/PuzzleDoorBP/BP_DoorDiscSlot.Left / Centre / Right` "Centre" _output_get_2)
  (bind _asbp_door_disc_slot_3 (cast `/Game/PuzzleDoor/PuzzleDoorBP/BP_DoorDiscSlot` (`ChildActorComponent.ChildActor` (`self.(Child Actor) Disc Slot Right`))))
  (bind _output_get_3 (set `self.Disc (Right)` _asbp_door_disc_slot_3))
  (set `/Game/PuzzleDoor/PuzzleDoorBP/BP_DoorDiscSlot.Left / Centre / Right` "Right" _output_get_3))

(event `/Game/PuzzleDoor/PuzzleDoorBP/BPI_DoorUpdate.Update Symbol Output`
  (params (`Left / Centre / Right` :type String) (`Texture (Lines)` :type "Texture Object Reference") (`Texture (Dots)` :type "Texture Object Reference"))
  (`MaterialInstanceDynamic.SetTextureParameterValue` (`self.Dynamic Material Instance`) (`KismetStringLibrary.Conv_StringToName` (`KismetStringLibrary.Concat_StrStr` `Left / Centre / Right` " (Lines)")) `Texture (Lines)`)
  (`MaterialInstanceDynamic.SetTextureParameterValue` (`self.Dynamic Material Instance`) (`KismetStringLibrary.Conv_StringToName` (`KismetStringLibrary.Concat_StrStr` `Left / Centre / Right` " (Dots)")) `Texture (Dots)`)
  (bind _answer_is_correct_ (`self.Check Answer`))
  (`KismetSystemLibrary.PrintString` "Door Solved" _answer_is_correct_ true (struct :`R` 0.042388 :`G` 1.0 :`A` 1.0)))

(fn `Check Answer`
  (returns (`Answer Is Correct?` :type Boolean))
  (return (== (`KismetMathLibrary.Xor_Int64Int64` (`KismetMathLibrary.Xor_Int64Int64` (`.PuzzleValue_40_1014FD784AA2D9D6B2693F843D53E481` (break `/Game/PuzzleDisc/PuzzleDiscBP/Struct_PuzzleDisc` (`/Game/PuzzleDoor/PuzzleDoorBP/BP_DoorDiscSlot.Disc Data` (`self.Disc (Left)`)))) (`.PuzzleValue_40_1014FD784AA2D9D6B2693F843D53E481` (break `/Game/PuzzleDisc/PuzzleDiscBP/Struct_PuzzleDisc` (`/Game/PuzzleDoor/PuzzleDoorBP/BP_DoorDiscSlot.Disc Data` (`self.Disc (Centre)`))))) (`.PuzzleValue_40_1014FD784AA2D9D6B2693F843D53E481` (break `/Game/PuzzleDisc/PuzzleDiscBP/Struct_PuzzleDisc` (`/Game/PuzzleDoor/PuzzleDoorBP/BP_DoorDiscSlot.Disc Data` (`self.Disc (Right)`))))) (`self.Door Passcode`))))

(fn `UserConstructionScript`
  (bind _returnvalue (`PrimitiveComponent.CreateDynamicMaterialInstance` (`self.Symbol Output`) 0 "/Game/PuzzleDoor/DoorMaterials/M_DoorSymbolOutput.M_DoorSymbolOutput" "None"))
  (set `self.Dynamic Material Instance` _returnvalue))