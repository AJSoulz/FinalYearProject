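; A puzzle door slot actor that holds a symbol disc the first-person player inserts or takes back.
; Interacting either stores the held disc's data and removes it from the player, or returns the stored disc, swapping the symbol texture to match.
; Each change notifies the owning doorway, assigned with a slot number through SetDoorwayReference.
; A dynamic material instance made in the construction script also drives a highlight while looked at.
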(event `/Game/FirstPersonBP/Blueprints/BPI_Interaction.Interact with Door Slot`
  (params (`Item Data` :type "/Game/PuzzleDisc/PuzzleDiscBP/Struct_PuzzleDisc Structure"))
  (if (`self.Is Slot Empty?`)
    (if (!= (`.ID_50_DEE222C7444A4711C8270282DCEC79DA` (break `/Game/PuzzleDisc/PuzzleDiscBP/Struct_PuzzleDisc` `Item Data`)) "None")
      (bind _output_get (set `self.Disc Data` `Item Data`))
      (set `self.Is Slot Empty?` false)
      (`MaterialInstanceDynamic.SetTextureParameterValue` (`self.Dynamic Material Instance`) "Symbol Texture" (`.SymbolTexture_42_12171B574ABD2CDDA975598A02914209` (break `/Game/PuzzleDisc/PuzzleDiscBP/Struct_PuzzleDisc` _output_get)))
      (bind _asfirst_person_character (cast `/Game/FirstPersonBP/Blueprints/FirstPersonCharacter` (`GameplayStatics.GetPlayerCharacter` 0)))
      (`/Game/FirstPersonBP/Blueprints/FirstPersonCharacter.Remove Disc` _asfirst_person_character)
      (message `/Game/PuzzleDoor/PuzzleDoorBP/BPI_DoorUpdate.Update Symbol Output` (`self.Doorway Reference`) (`self.Doorway Slot Number`) false)
      (else
        (`KismetSystemLibrary.PrintString` "Hand is empty" true true (struct :`R` 1.0 :`G` 0.948471 :`A` 1.0))))
    (else
      (set `self.Is Slot Empty?` true)
      (`MaterialInstanceDynamic.SetTextureParameterValue` (`self.Dynamic Material Instance`) "Symbol Texture" "/Game/PuzzleDisc/SymbolTextures/T_Symbol_0000000000000.T_Symbol_0000000000000")
      (bind _asfirst_person_character_2 (cast `/Game/FirstPersonBP/Blueprints/FirstPersonCharacter` (`GameplayStatics.GetPlayerCharacter` 0)))
      (message `/Game/Inventory/BPI_ItemPickup.OnItemPickup` _asfirst_person_character_2 (`self.Disc Data`))
      (set `self.Disc Data` (struct))
      (message `/Game/PuzzleDoor/PuzzleDoorBP/BPI_DoorUpdate.Update Symbol Output` (`self.Doorway Reference`) (`self.Doorway Slot Number`) true))))

(event `/Game/FirstPersonBP/Blueprints/BPI_Interaction.Now Looking At`
  (`MaterialInstanceDynamic.SetScalarParameterValue` (`self.Dynamic Material Instance`) "Highlight" 1.0))

(event `/Game/FirstPersonBP/Blueprints/BPI_Interaction.No Longer Looking At`
  (`MaterialInstanceDynamic.SetScalarParameterValue` (`self.Dynamic Material Instance`) "Highlight" 0.0))

(fn `Set Doorway Reference`
  (params (`Doorway Reference` :type "/Game/PuzzleDoor/PuzzleDoorBP/BP_Doorway Object Reference") (`Slot Number` :type Integer))
  (set `self.Doorway Reference` `Doorway Reference`)
  (set `self.Doorway Slot Number` `Slot Number`))

(fn `UserConstructionScript`
  (bind _returnvalue (`PrimitiveComponent.CreateDynamicMaterialInstance` (`self.Disc Slot Mesh`) 0 "/Game/PuzzleDoor/DoorMaterials/M_DoorSlot.M_DoorSlot" "None"))
  (set `self.Dynamic Material Instance` _returnvalue))