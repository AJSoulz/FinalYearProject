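; Puzzle disc pickup that the first-person player collects, reviving the skeletons it downed.
; On BeginPlay it loads its item data and face material from a data table, then plays a timeline that raises, scales and spins it.
; Overlap events stay off until that animation finishes.
; Player overlap sends the item data to the character and to skeletons tagged with the disc's ID, then destroys the disc.
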(event `self.ReceiveBeginPlay`
  (bind _start_location (`self.Start Location`))
  (set `PrimitiveComponent.bGenerateOverlapEvents` false (`self.SphereCollision`))
  (bind _returnvalue (`|GetDataTableRow` "/Game/PuzzleDisc/PuzzleDiscBP/DataTable_PuzzleDisc.DataTable_PuzzleDisc" (`self.Data Table Row`))
    (:`then`
      (bind _output_get (set `self.ItemData` _returnvalue))
      (bind ((`MaterialInstance_41_B9B57ED740E93DD13ED561B720CFAD3D` _materialinstance)) (break `/Game/PuzzleDisc/PuzzleDiscBP/Struct_PuzzleDisc` _output_get))
      (`PrimitiveComponent.SetMaterial` (`self.Obverse`) 0 _materialinstance)
      (`PrimitiveComponent.SetMaterial` (`self.Reverse`) 0 _materialinstance)
      (set `self.Start Location` (`self.K2_GetActorLocation`))
      (bind (_direction _height _scale _rotation) (`Timeline|Respawn Animation`)
        (:`Update`
          (`self.K2_SetActorLocation` (`KismetMathLibrary.VLerp` _start_location (+ _start_location (0.0 0.0 100.0)) _height))
          (`self.SetActorScale3D` (`KismetMathLibrary.MakeVector` _scale _scale (.z (`self.GetActorScale3D`))))
          (`self.K2_SetActorRotation` (`KismetMathLibrary.RLerp` (struct) (struct :`Yaw` 585.0 :`Roll` 45.0) _rotation)))
        (:`Finished`
          (set `PrimitiveComponent.bGenerateOverlapEvents` true (`self.SphereCollision`)))))))

(event `self.SphereCollision.OnComponentBeginOverlap`
  (params (OverlappedComponent :type "PrimitiveComponent Object Reference") (OtherActor :type "Actor Object Reference") (OtherComp :type "PrimitiveComponent Object Reference") (OtherBodyIndex :type Integer) (bFromSweep :type Boolean) (SweepResult :type "HitResult Structure (by ref)"))
  (bind _itemdata (`self.ItemData`))
  (bind _asfirst_person_character (cast `/Game/FirstPersonBP/Blueprints/FirstPersonCharacter` OtherActor)) ; Ensure that it is picked up by the player.
  (message `/Game/Inventory/BPI_ItemPickup.OnItemPickup` _asfirst_person_character _itemdata) ; Notify FirstPersonCharacter.\nWill add this PuzzleDisc to the player inventory.
  (bind _outactors (`GameplayStatics.GetAllActorsOfClassWithTag` "/Game/Enemies/Skeleton/BP_Skeleton.BP_Skeleton_C" (`.ID_50_DEE222C7444A4711C8270282DCEC79DA` (break `/Game/PuzzleDisc/PuzzleDiscBP/Struct_PuzzleDisc` _itemdata))))
  (message `/Game/Inventory/BPI_ItemPickup.OnItemPickup` _outactors (`self.ItemData`)) ; Notify all Skeletons downed by this disc. \nThey will all get back up.
  (`self.K2_DestroyActor`))

(fn `UserConstructionScript`)